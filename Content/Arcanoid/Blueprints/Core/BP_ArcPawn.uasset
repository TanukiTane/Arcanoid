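; Player paddle pawn for an Arkanoid-style game that launches balls, tracks lives and score, and applies pickup bonuses.
; SpawnBall allows one main ball while lives remain; its destruction costs a life and calls game end at zero.
; Overlapped bonuses add score and either widen the paddle, grant a life or spawn a smaller, untracked extra ball.
; Widening stacks, and a retriggerable delay restores the scale saved at BeginPlay.
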(event OnComponentBeginOverlap(Cube)
  (params (OverlappedComponent :type Primitive%20Component%20Object%20Reference) (OtherActor :type Actor%20Object%20Reference) (OtherComp :type Primitive%20Component%20Object%20Reference) (OtherBodyIndex :type Integer) (bFromSweep :type Boolean) (SweepResult :type Hit%20Result%20Structure%20%28by%20ref%29))
  ;[1 1 1] Bonus Logic for Pawn
  (bind _asbp_bonus (Utilities|Casting|CastToBP_Bonus OtherActor))
  (switch Utilities|FlowControl|Switch|SwitchonE_BonusType (Variables|/Game/Arcanoid/Blueprints/Bonuses/BP_Bonus.BP_Bonus_C|GetBonusType _asbp_bonus)
    (:NewEnumerator0
      (CallFunction|MaxEvent))
    (:NewEnumerator1
      (CallFunction|LiveEvent))
    (:NewEnumerator2
      (CallFunction|BallEvent)))
  (CallFunction|AddScore 50)
  (Actor|DestroyActor _asbp_bonus))

(event Custom|SpawnBall
  ;[1 1 1] SpawnBall By key
  (if (> (Variables|Default|GetPlayerLive) 0)
    (Variables|Default|GetAliveBall
      (:then)
      (:else
        (bind _returnvalue (Game|SpawnActorfromClass "/Game/Arcanoid/Blueprints/BP_Ball.BP_Ball_C" (Math|Transform|MakeTransform (Transformation|GetWorldLocation (Variables|Default|GetArrow))) "Undefined" 0 0))
        (bind _output_get (Variables|Default|SetAliveBall _returnvalue))
        (Game|BindEventtoOnDestroyed _output_get (delegate Custom|BallsDeath))))))

(event Custom|BallsDeath
  (params (DestroyedActor :type Actor%20Object%20Reference))
  ;[1 1 1] HealthChange
  (bind _result (Math|Integer|DecrementInt (Variables|Default|GetPlayerLive))
    (:%20%20
      (Default|CallLivesChanged _result)
      (if (<= _result 0)
        (Default|CallGameEnd)))))

(event Custom|MaxEvent
  (bind _cube (Variables|Default|GetCube))
  (bind _relativescale3d (Variables|/Script/Engine.SceneComponent|GetRelativeScale3D _cube))
  ;[1 1 1] Event for MaxBonus
  (Transformation|SetRelativeScale3D _cube (Math|Vector|MakeVector (.x _relativescale3d) (* (.y _relativescale3d) 1.2) (.z _relativescale3d)))
  (CallFunction|MinEvent))

(event Custom|LiveEvent
  ;[1 1 1] Event for Live Bonus +1Live
  (bind _result (Math|Integer|IncrementInt (Variables|Default|GetPlayerLive))
    (:%20%20
      (Default|CallLivesChanged _result))))

(event Custom|BallEvent
  ;[1 1 1] Event for BallBonus - Spawn second Ball
  (Game|SpawnActorfromClass "/Game/Arcanoid/Blueprints/BP_Ball.BP_Ball_C" (Math|Transform|MakeTransform (Transformation|GetWorldLocation (Variables|Default|GetArrow)) "0, 0, 0" "0.500000,0.500000,0.500000") "Undefined" 0 0))

(event Custom|MinEvent
  ;[1 1 1] Set Default scale after 6 sec
  (Utilities|FlowControl|RetriggerableDelay 6.0)
  (Transformation|SetRelativeScale3D (Variables|Default|GetCube) (Variables|Default|GetDefaultScale)))

(event EventBeginPlay
  (Variables|Default|SetDefaultScale (Variables|/Script/Engine.SceneComponent|GetRelativeScale3D (Variables|Default|GetCube))))

(fn ConstructionScript)

(fn AddScore
  (params (Ammount :type Integer))
  (bind _output_get (Variables|Default|SetScore (+ (Variables|Default|GetScore) (Math|Integer|Absolute(Integer) Ammount))))
  (Default|CallScoreChange _output_get))