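; Player controller for the Arcanoid game that owns the HUD, moves the paddle pawn and handles game end.
; On possess it binds the pawn's game-end event, and on BeginPlay it creates the HUD and binds the cube generator's all-cubes-destroyed event.
; Both events show the same win screen and switch to UI input.
; Axis input slides the pawn sideways with a swept offset, and an action spawns the ball.
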(event Custom|GameFinished
  ;[1 1 1] Call Widget WinScreen
  (Widget|SetVisibility (Variables|Default|GetHUD) "Collapsed")
  (bind _returnvalue (UserInterface|CreateWidget "/Game/Arcanoid/UI/Menu/WBP_WinScreen.WBP_WinScreen_C" self))
  (UserInterface|Viewport|AddtoViewport _returnvalue 0)
  (Input|SetInputModeUIOnly self 0 "LockOnCapture" false)
  (Variables|Default|SetbShowMouseCursor true))

(event EventBeginPlay
  (Utilities|FlowControl|Sequence
    (:then_0
      ;[1 1 1] Call UI
      (Input|SetInputModeGameOnly self false)
      (bind _returnvalue (UserInterface|CreateWidget "/Game/Arcanoid/UI/Widget/WBP_HUD.WBP_HUD_C" self))
      (bind _output_get (Variables|Default|SetHUD _returnvalue))
      (UserInterface|Viewport|AddtoViewport _output_get 0))
    (:then_1
      (bind _returnvalue_2 (Actor|GetActorOfClass "/Game/Arcanoid/Blueprints/BP_CubeGenerator.BP_CubeGenerator_C"))
      (EventDispatchers|BindEventtoAllCubesDestroy _returnvalue_2 (delegate Custom|GameFinished)))))

(event EventTick
  (params (DeltaSeconds :type Float%20%28single-precision%29)))

(event EventPossess
  (params (PossessedPawn :type Pawn%20Object%20Reference))
  (bind _asbp_arc_pawn (Utilities|Casting|CastToBP_ArcPawn PossessedPawn))
  (bind _output_get (Variables|Default|SetPlayerPawn _asbp_arc_pawn))
  (EventDispatchers|BindEventtoGameEnd _output_get (delegate Custom|GameFinished)))

(event Input|ActionEvents|InputActionSpawnBall
  (params (Key :type Key%20Structure :default "None"))
  ;[1 1 1] Input ball spawn
  (:Pressed
    (Default|SpawnBall (Variables|Default|GetPlayerPawn))))

(event Input|AxisEvents|InputAxisLeftRight
  (params (AxisValue :type Float%20%28single-precision%29))
  ;[1 1 1] Input Move
  (Transformation|AddActorWorldOffset (Variables|Default|GetPlayerPawn) (Math|Vector|MakeVector 0.0 (* AxisValue (Utilities|Time|GetWorldDeltaSeconds) (Variables|Default|GetSpeed)) 0.0) true))

(fn ConstructionScript)