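; BP_CubeGenerator is an Arcanoid level actor that builds the grid of breakable cubes and tracks when all are destroyed.
; The construction script previews the X/Y grid, spaced by Padding, with static mesh components.
; BeginPlay swaps the preview for spawned BP_CubeChild actors and binds their death events.
; Each death adds score to BP_ArcPawn, and the AllCubesDestroy dispatcher fires once the count reaches the spawned total.
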(event Custom|CubeDeath
  (params (Score :type Integer))
  ;[1 1 1] Write Score
  (Default|AddScore (Variables|Default|GetArcPawn) Score)
  (Math|Integer|IncrementInt (Variables|Default|GetDeadCube)
    (:%20%20
      (if (>= (Variables|Default|GetDeadCube) (Variables|Default|GetAmmount%20CubesForWin))
        (Default|CallAllCubesDestroy)))))

(event EventBeginPlay
  (bind _returnvalue (Transformation|GetActorLocation))
  (Utilities|FlowControl|Sequence
    (:then_0
      (bind _returnvalue_2 (Actor|GetActorOfClass "/Game/Arcanoid/Blueprints/Core/BP_ArcPawn.BP_ArcPawn_C"))
      (Variables|Default|SetArcPawn _returnvalue_2))
    (:then_1
      ;[1 1 1] Destroy Scale
      (for _array_element (Variables|Default|GetPreview%20Array)
        (Components|DestroyComponent _array_element))
      ;[1 1 1] Spawn Actor Cubes in Scale
      (for _index (range 0 (Variables|Default|GetY))
        (for _index_2 (range 0 (Variables|Default|GetX))
          (bind _returnvalue_3 (Game|SpawnActorfromClass "/Game/Arcanoid/Blueprints/BP_CubeChild.BP_CubeChild_C" (Math|Transform|MakeTransform (Math|Vector|MakeVector (+ (+ (.x _returnvalue) (Math|Conversions|ToFloat(Integer) (* _index_2 (Variables|Default|GetPadding)))) 5e+01) (+ (+ (.y _returnvalue) (Math|Conversions|ToFloat(Integer) (* _index (Variables|Default|GetPadding)))) 5e+01) (+ (.z _returnvalue) 3e+01))) "Undefined" 0 0))
          (Utilities|Array|Add (Variables|Default|GetCubesArray) _returnvalue_3)))
      ;[1 1 1] Write Score
      (bind _ammountcubes (CallFunction|GetCubesforWin))
      (Variables|Default|SetAmmount%20CubesForWin _ammountcubes)
      (for _array_element_2 (Variables|Default|GetCubesArray)
        (EventDispatchers|BindEventtoCubeDead _array_element_2 (delegate Custom|CubeDeath))))))

(fn ConstructionScript
  ;[1 1 1] Generate scale for BP_Cubes
  (for _index (range 0 (Variables|Default|GetY))
    (for _index_2 (range 0 (Variables|Default|GetX))
      (bind _returnvalue (AddComponent|AddStaticMeshComponent false (Math|Transform|MakeTransform (Math|Vector|MakeVector (Math|Conversions|ToFloat(Integer) (* _index_2 (Variables|Default|GetPadding))) (Math|Conversions|ToFloat(Integer) (* _index (Variables|Default|GetPadding))) 0.0))))
      (Utilities|Array|Add (Variables|Default|GetPreview%20Array) _returnvalue))))

(fn GetCubesforWin
  (return (Utilities|Array|Length (Variables|Default|GetCubesArray))))