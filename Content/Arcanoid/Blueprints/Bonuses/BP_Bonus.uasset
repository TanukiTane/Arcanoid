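; BP_Bonus is a bonus actor for the Arcanoid game that travels in a straight line and displays its bonus type.
; The construction script randomly picks one of three BonusType values and writes its name to a TextRender component.
; Tick applies a frame-rate independent, swept world offset along Direction at Speed, using only the X and Y components.
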(event EventTick
  (params (DeltaSeconds :type Float%20%28single-precision%29))
  (bind _speed (Variables|Default|GetSpeed))
  (bind _direction (Variables|Default|GetDirection))
  (bind _returnvalue (* DeltaSeconds _speed))
  (bind _returnvalue_2 (* _direction _returnvalue))
  ;[1 1 1] Actor Movement
  (Transformation|AddActorWorldOffset (Math|Vector|MakeVector (.x _returnvalue_2) (.y _returnvalue_2) 0.0) true))

(fn ConstructionScript
  (Variables|Default|SetBonusType (Utilities|Select :Index (Math|Random|RandomIntegerinRange 0 2) :Option%200 "NewEnumerator0" :Option%201 "NewEnumerator1" :Option%202 "NewEnumerator2"))
  (Rendering|Components|TextRender|SetText (Variables|Default|GetTextRender) (Utilities|Text|ToText(String) (Utilities|String|EnumtoString (Variables|Default|GetBonusType)))))