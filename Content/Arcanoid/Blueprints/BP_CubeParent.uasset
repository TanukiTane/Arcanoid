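; Parent Blueprint for Arcanoid cubes, breakable targets that lose a life each time a BP_Ball hits them.
; The construction script randomizes Lives from one to five and sets a matching metal material and score, with the top three tiers sharing yellow.
; Each hit decrements Lives and updates the material; at zero, the cube fires the CubeDead dispatcher with its Score and destroys itself.
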(event Custom|BallIsHit
  (bind _cube (Variables|Default|GetCube))
  ;[1 1 1] Switch Lives
  (bind _result (Math|Integer|DecrementInt (Variables|Default|GetLives))
    (:%20%20
      (if (<= _result 0)
        ;[1 1 1] Destroy if lives =0, change MI_Color, if chnge lives
        (Default|CallCubeDead (Variables|Default|GetScore))
        (Actor|DestroyActor)
        (else
          (switch int (Variables|Default|GetLives)
            (:1
              (Rendering|Material|SetMaterial _cube 0 "/Game/Arcanoid/Materials/Metals/MI_MetalRed.MI_MetalRed"))
            (:2
              (Rendering|Material|SetMaterial _cube 0 "/Game/Arcanoid/Materials/Metals/MI_MetalWhite.MI_MetalWhite"))
            (:3
              (Rendering|Material|SetMaterial _cube 0 "/Game/Arcanoid/Materials/Metals/MI_MetalYellow.MI_MetalYellow" :!label _label))
            (:4
              (goto _label))
            (:5
              (goto _label))))))))

(event Collision|EventHit
  (params (MyComp :type Primitive%20Component%20Object%20Reference) (Other :type Actor%20Object%20Reference) (OtherComp :type Primitive%20Component%20Object%20Reference) (bSelfMoved :type Boolean) (HitLocation :type Vector :default "0, 0, 0") (HitNormal :type Vector :default "0, 0, 0") (NormalImpulse :type Vector :default "0, 0, 0") (Hit :type Hit%20Result%20Structure%20%28by%20ref%29))
  (Utilities|Casting|CastToBP_Ball Other)
  (CallFunction|BallIsHit))

(event EventBeginPlay)

(event EventTick
  (params (DeltaSeconds :type Float%20%28single-precision%29)))

(fn ConstructionScript
  (bind _cube (Variables|Default|GetCube))
  (bind _output_get (Variables|Default|SetLives (Math|Random|RandomIntegerinRange 1 5)))
  (switch int _output_get
    (:1
      (Rendering|Material|SetMaterial _cube 0 "/Game/Arcanoid/Materials/Metals/MI_MetalRed.MI_MetalRed")
      (Variables|Default|SetScore 100))
    (:2
      (Rendering|Material|SetMaterial _cube 0 "/Game/Arcanoid/Materials/Metals/MI_MetalWhite.MI_MetalWhite")
      (Variables|Default|SetScore 200))
    (:3
      (Rendering|Material|SetMaterial _cube 0 "/Game/Arcanoid/Materials/Metals/MI_MetalYellow.MI_MetalYellow" :!label _label)
      (Variables|Default|SetScore 400))
    (:4
      (goto _label))
    (:5
      (goto _label))))