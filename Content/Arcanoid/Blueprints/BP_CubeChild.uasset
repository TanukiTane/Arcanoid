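; BP_CubeChild is a child cube Blueprint for the Arcanoid game that can drop a bonus when destroyed.
; On BeginPlay it checks whether its material is MI_MetalWhite and, if so, binds a spawn event to its OnDestroyed delegate.
; That event spawns BP_Bonus at the cube's location with a fixed rotation, while ball hits and construction defer to the parent class.
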(event Custom|SpawnBonus
  (params (DestroyedActor :type Actor%20Object%20Reference))
  ;[1 1 1] Event on Destroy Cube
  (Game|SpawnActorfromClass "/Game/Arcanoid/Blueprints/Bonuses/BP_Bonus.BP_Bonus_C" (Math|Transform|MakeTransform (Transformation|GetActorLocation) "90.000000,0.000000,0.000000") "AlwaysSpawn" 0 0))

(event EventBeginPlay
  ;[1 1 1] Event on Destroy Cube
  ;;[1 1 1] Condition  of bonus spawn
  (if (== (Rendering|Material|GetMaterial (Variables|Default|GetCube) 0) "/Game/Arcanoid/Materials/Metals/MI_MetalWhite.MI_MetalWhite")
    (Game|BindEventtoOnDestroyed (delegate Custom|SpawnBonus))))

(event EventBallIsHit
  (|CallParentFunction))

(fn ConstructionScript
  (|CallParentFunction))